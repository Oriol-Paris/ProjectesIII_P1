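; BP_dynamicenemy is an enemy actor with a health bar widget that never dies from damage.
; BeginPlay caches the HP_bar user widget, seeds its max and current health, and plays a sound at the enemy's location.
; Each AIDamage event subtracts a fixed amount of health and updates the bar, while Tick refills health once it drops to a low threshold without refreshing the bar.
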(event Collision|EventActorBeginOverlap
  (params (OtherActor :type Actor%20Object%20Reference)))

(event EventTick
  (params (DeltaSeconds :type Float%20%28single-precision%29))
  (if (<= (Variables|Default|GetCurrenthp) 5.0)
    (Variables|Default|SetCurrenthp 1e+02)))

(event EventAIDamage
  (Variables|Default|SetCurrenthp (- (Variables|Default|GetCurrenthp) 5.0))
  (Variables|/Game/EDU/widgets/HP_bar.HP_bar_C|Setcurrent%20health (Variables|Default|GetAs%20HP%20Bar) (Variables|Default|GetCurrenthp)))

(event EventBeginPlay
  (Utilities|FlowControl|Sequence
    (:then_0
      (bind _ashp_bar (Utilities|Casting|CastToHP_bar (UserInterface|GetUserWidgetObject (Variables|Default|GetWidget))))
      (Variables|Default|SetAs%20HP%20Bar _ashp_bar)
      (Variables|/Game/EDU/widgets/HP_bar.HP_bar_C|Setmax%20health _ashp_bar (Variables|Default|GetMax%20hp))
      (Variables|/Game/EDU/widgets/HP_bar.HP_bar_C|Setcurrent%20health _ashp_bar (Variables|Default|GetCurrenthp)))
    (:then_1
      (Audio|PlaySoundatLocation "/Game/EDU/MS_xieheeeeeehuahuapiaochinhehuaopiaooooxinhuee.MS_xieheeeeeehuahuapiaochinhehuaopiaooooxinhuee" (Transformation|GetActorLocation) "0, 0, 0" 1.0 1.0 0.0 0 0 0 0))))

(fn ConstructionScript)