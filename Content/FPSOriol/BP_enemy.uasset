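; Enemy actor with a health bar widget and a skeletal mesh that continuously cycles through rainbow colors.
; BeginPlay fills the HP_bar widget, then creates a dynamic material whose Color parameter a self-calling, delay-chained ChangeColor event steps through.
; AIDamage subtracts fixed damage and updates the bar.
; Tick resets low health to a hard-coded full value instead of killing the enemy, without updating the bar.
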(event Custom|Change%20color
  (Rendering|Material|SetVectorParameterValue (Variables|Default|GetDynamicMaterialç) "Color" "(R=1.000000,G=0.000000,B=0.024272,A=1.000000)" :!class /Script/Engine.MaterialInstanceDynamic)
  (Utilities|FlowControl|Delay 0.2)
  (Rendering|Material|SetVectorParameterValue (Variables|Default|GetDynamicMaterialç) "Color" "(R=1.000000,G=0.360515,B=0.000000,A=1.000000)" :!class /Script/Engine.MaterialInstanceDynamic)
  (Utilities|FlowControl|Delay 0.2)
  (Rendering|Material|SetVectorParameterValue (Variables|Default|GetDynamicMaterialç) "Color" "(R=1.000000,G=0.729092,B=0.000000,A=1.000000)" :!class /Script/Engine.MaterialInstanceDynamic)
  (Utilities|FlowControl|Delay 0.2)
  (Rendering|Material|SetVectorParameterValue (Variables|Default|GetDynamicMaterialç) "Color" "(R=0.171052,G=1.000000,B=0.000000,A=1.000000)" :!class /Script/Engine.MaterialInstanceDynamic)
  (Utilities|FlowControl|Delay 0.2)
  (Rendering|Material|SetVectorParameterValue (Variables|Default|GetDynamicMaterialç) "Color" "(R=0.000000,G=0.122017,B=1.000000,A=1.000000)" :!class /Script/Engine.MaterialInstanceDynamic)
  (Utilities|FlowControl|Delay 0.2)
  (Rendering|Material|SetVectorParameterValue (Variables|Default|GetDynamicMaterialç) "Color" "(R=0.903122,G=0.000000,B=1.000000,A=1.000000)" :!class /Script/Engine.MaterialInstanceDynamic)
  (Utilities|FlowControl|Delay 0.2)
  (CallFunction|ChangeColor))

(event Collision|EventActorBeginOverlap
  (params (OtherActor :type Actor%20Object%20Reference)))

(event EventTick
  (params (DeltaSeconds :type Float%20%28single-precision%29))
  (if (<= (Variables|Default|GetCurrenthp) 5.0)
    (Variables|Default|SetCurrenthp 1e+02)))

(event EventAIDamage
  (Variables|Default|SetCurrenthp (- (Variables|Default|GetCurrenthp) 5.0))
  (Variables|/Game/EDU/widgets/HP_bar.HP_bar_C|Setcurrent%20health (Variables|Default|GetAs%20HP%20Bar) (Variables|Default|GetCurrenthp)))

(event EventBeginPlay
  (Utilities|FlowControl|Sequence
    (:then_0
      (bind _ashp_bar (Utilities|Casting|CastToHP_bar (UserInterface|GetUserWidgetObject (Variables|Default|GetWidget))))
      (Variables|Default|SetAs%20HP%20Bar _ashp_bar)
      (Variables|/Game/EDU/widgets/HP_bar.HP_bar_C|Setmax%20health _ashp_bar (Variables|Default|GetMax%20hp))
      (Variables|/Game/EDU/widgets/HP_bar.HP_bar_C|Setcurrent%20health _ashp_bar (Variables|Default|GetCurrenthp)))
    (:then_1
      (bind _returnvalue (Rendering|Material|CreateDynamicMaterialInstance (Rendering|Material|GetMaterial (Variables|Default|GetSkeletalMesh) 0) "None" "None" :!class /Script/Engine.KismetMaterialLibrary))
      (bind _output_get (Variables|Default|SetDynamicMaterialç _returnvalue))
      (Rendering|Material|SetMaterial (Variables|Default|GetSkeletalMesh) 0 _output_get))
    (:then_2
      (CallFunction|ChangeColor))))

(fn ConstructionScript)